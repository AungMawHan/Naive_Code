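; Player character Blueprint that handles movement, mouse look, HUD creation and passive Health and Mana regeneration.
; Move axes follow the control rotation's yaw only, turn axes feed controller yaw and pitch, and BeginPlay adds the RpgHUD widget to the viewport.
; Tick drives two independent Delay nodes as repeating timers, each adding regen at its own rate and capping the normalized value at full.
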(event EventBeginPlay
  ;[1 1 1] Health&TimeSpaceBarWidget
  (bind _returnvalue (UserInterface|CreateWidget "/Game/CustomBP/RpgHUD.RpgHUD_C"))
  (UserInterface|Viewport|AddtoViewport _returnvalue 0))

(event EventTick
  (params (DeltaSeconds :type Float%20%28single-precision%29))
  ;[1 1 1] EveryTick
  (Utilities|FlowControl|Sequence
    (:then_0
      ;[1 1 1] HealthRegen
      (Utilities|FlowControl|Delay (Variables|Default|GetHealthRate))
      (if (< (Variables|Default|GetHealth) 1.0)
        (Variables|Default|SetHealth (+ (Variables|Default|GetHealth) (Variables|Default|GetHealthRegen)))
        (if (>= (Variables|Default|GetHealth) 1.0)
          (Variables|Default|SetHealth 1.0))))
    (:then_1
      ;[1 1 1] ManaRegen
      (Utilities|FlowControl|Delay (Variables|Default|GetManaRate))
      (if (< (Variables|Default|GetMana) 1.0)
        (Variables|Default|SetMana (+ (Variables|Default|GetMana) (Variables|Default|GetManaRegen)))
        (if (>= (Variables|Default|GetMana) 1.0)
          (Variables|Default|SetMana 1.0))))))

(event Input|AxisEvents|InputAxisMoveForward
  (params (AxisValue :type Float%20%28single-precision%29))
  ;[1 1 1] Movement
  (Pawn|Input|AddMovementInput (Math|Vector|GetForwardVector (Math|Rotator|MakeRotator 0.0 0.0 (.Yaw (Math|Rotator|BreakRotator (Pawn|GetControlRotation :!class /Script/Engine.Pawn))))) AxisValue false))

(event Input|AxisEvents|InputAxisMoveRight
  (params (AxisValue :type Float%20%28single-precision%29))
  ;[1 1 1] Movement
  (Pawn|Input|AddMovementInput (Math|Vector|GetRightVector (Math|Rotator|MakeRotator 0.0 0.0 (.Yaw (Math|Rotator|BreakRotator (Pawn|GetControlRotation :!class /Script/Engine.Pawn))))) AxisValue false))

(event Input|AxisEvents|InputAxisTurnUp
  (params (AxisValue :type Float%20%28single-precision%29))
  ;[1 1 1] MouseTurn
  (Pawn|Input|AddControllerPitchInput AxisValue))

(event Input|AxisEvents|InputAxisTurnRight
  (params (AxisValue :type Float%20%28single-precision%29))
  ;[1 1 1] MouseTurn
  (Pawn|Input|AddControllerYawInput AxisValue))

(fn ConstructionScript)